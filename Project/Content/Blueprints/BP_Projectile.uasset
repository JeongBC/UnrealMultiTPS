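; BP_Projectile is an actor that explodes on a fixed one-second timer after spawning.
; BeginPlay waits out the delay and calls Explode, with no collision or hit trigger in its graphs.
; Explode spawns the P_Explosion particle effect, applies radial damage credited to the instigator's controller, and destroys the actor.
; A debug sphere drawn after the destroy call shows the blast radius, which comes from the variable NewVar0.
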(event Custom|Explode
  (bind _returnvalue (Transformation|GetActorLocation))
  ;[1 1 1] Make C++ CODE
  (Effects|SpawnEmitteratLocation "/Game/WeaponEffects/Explosion/P_Explosion.P_Explosion" _returnvalue)
  (Game|Damage|ApplyRadialDamage 1e+02 _returnvalue (Variables|Default|GetNewVar_0) 0 0 self (Game|GetInstigatorController) false "ECC_Visibility")
  (Actor|DestroyActor)
  (Rendering|Debug|DrawDebugSphere _returnvalue (Variables|Default|GetNewVar_0) 12 "(R=1.000000,G=0.110346,B=0.000000,A=1.000000)" 2.0 2.0))

(event EventBeginPlay
  ;[1 1 1] Make C++ CODE
  (Utilities|FlowControl|Delay 1.0)
  (CallFunction|Explode))

(fn ConstructionScript)