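; BP_BattleMode is a battle mode Blueprint with logic for spawning tracker bots and scoring kills, currently left disconnected.
; The EQS_FindSpawn query handler spawns BP_TrackerBot at each result location with a debug sphere.
; The kill handler calls AddScore with zero on the killer's JPlayerState when the victim pawn is not player-controlled, then prints the score.
; BeginPlay and SpawnNewBot are empty, so neither the query nor either delegate binding runs.
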(event Custom|OnQueryFinishedEvent_이벤트_0
  (params (QueryInstance :type Env%20Query%20Instance%20Blueprint%20Wrapper%20Object%20Reference) (QueryStatus :type EEnvQueryStatus%20Enum :default "Processing"))
  (switch Utilities|FlowControl|Switch|SwitchonEEnvQueryStatus QueryStatus
    (:Success
      (for _array_element (Class|EnvQueryInstanceBlueprintWrapper|GetResultsasLocations QueryInstance)
        (Rendering|Debug|DrawDebugSphere _array_element 5e+01 12 "(R=1.000000,G=0.592491,B=0.020335,A=1.000000)" 2.0 2.0)
        (Game|SpawnActorfromClass "/Game/Blueprints/AI/BP_TrackerBot.BP_TrackerBot_C" (Math|Transform|MakeTransform _array_element) "AdjustIfPossibleButDontSpawnIfColliding" 0 0)))))

(event Custom|OnActorKilled_이벤트_0
  (params (VictimActor :type Actor%20Object%20Reference) (KillerActor :type Actor%20Object%20Reference) (KillerController :type Controller%20Object%20Reference))
  (bind _aspawn (Utilities|Casting|CastToPawn VictimActor))
  (if (not (Pawn|IsPlayerControlled _aspawn))
    (bind _asjplayer_state (Utilities|Casting|CastToJPlayerState (Variables|/Script/Engine.Pawn|GetPlayerState (Pawn|GetControlledPawn KillerController))))
    (Class|JPlayerState|AddScore _asjplayer_state 0.0)
    (Development|PrintString (Utilities|String|ToString(Float) (Variables|/Script/Engine.PlayerState|GetScore _asjplayer_state)))))

(event EventBeginPlay)

(event EventSpawnNewBot)

(fn ConstructionScript)